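; BP_guard is a guard Blueprint that shows dialogue lines in a WB_Dialouge widget.
; Each Talk event increments Talkindex and, while it is within the Dialogue array, writes that entry to the widget's TalkText.
; The widget is created and added to the viewport if the stored reference is invalid, then removed from its parent when the index passes the last line.
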(event `/Game/Dialouge/BP_Dialouge.Talk`
  (`/Engine/EditorBlueprintResources/StandardMacros.IncrementInt` (`self.talkindex`)
    (:`  `
      (if (< (`self.talkindex`) (`KismetArrayLibrary.Array_Length` (`self.Dialogue`)))
        (`self.NewVar`
          (:`then`
            _)
          (:`else`
            (bind _returnvalue (`|CreateWidget` "/Game/Dialouge/WB_Dialouge.WB_Dialouge_C" (`GameplayStatics.GetPlayerController` 0)))
            (bind _output_get (set `self.NewVar` _returnvalue))
            (`UserWidget.AddToViewport` _output_get 0)))
        (`TextBlock.SetText` (`/Game/Dialouge/WB_Dialouge.TalkText` (`self.NewVar`)) (`KismetTextLibrary.Conv_StringToText` (`|GetArrayItem` (`self.Dialogue`) (`self.talkindex`))))
        (else
          (`Widget.RemoveFromParent` (`self.NewVar`)))))))

(fn `UserConstructionScript`)