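; Decoration prop Blueprint from an ArchVis pack, a music-themed deco static mesh with an adjustable material.
; The Construction Script creates a dynamic instance of M_AVP2_Deco on slot 0 and assigns the shared deco base color, mask and normal textures.
; It then passes the Deco color, metalness and roughness variables into that material.
; The event graph holds only disabled default events, so there is no runtime logic.
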(event `self.ReceiveBeginPlay`)

(event `self.ReceiveActorBeginOverlap`
  (params (OtherActor :type "Actor Object Reference")))

(event `self.ReceiveTick`
  (params (DeltaSeconds :type "Float (single-precision)")))

(fn `UserConstructionScript`
  (bind _returnvalue (`PrimitiveComponent.CreateDynamicMaterialInstance` (`self.StaticMesh`) 0 "/Game/ArchVisPolishPack02/Materials/M_AVP2_Deco.M_AVP2_Deco"))
  (`MaterialInstanceDynamic.SetTextureParameterValue` _returnvalue "Base Color Texture" "/Game/ArchVisPolishPack02/Textures/T_AVP2_Deco_D.T_AVP2_Deco_D")
  (`MaterialInstanceDynamic.SetTextureParameterValue` _returnvalue "Mask Texture" "/Game/ArchVisPolishPack02/Textures/T_AVP2_Deco_M.T_AVP2_Deco_M")
  (`MaterialInstanceDynamic.SetTextureParameterValue` _returnvalue "Normal Texture" "/Game/ArchVisPolishPack02/Textures/T_AVP2_Deco_N.T_AVP2_Deco_N")
  (`MaterialInstanceDynamic.SetScalarParameterValue` _returnvalue "Deco.Metalness" (`self.Deco.Metalness`))
  (`MaterialInstanceDynamic.SetScalarParameterValue` _returnvalue "Deco.Roughness" (`self.Deco.Roughness`))
  (`MaterialInstanceDynamic.SetVectorParameterValue` _returnvalue "Deco.Color" (`self.Deco.Color`)))