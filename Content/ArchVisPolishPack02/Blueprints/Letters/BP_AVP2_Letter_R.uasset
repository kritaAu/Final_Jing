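; BP_AVP2_Letter_R is an ArchVis Polish Pack 02 letter prop, by name the letter R, with an adjustable surface finish.
; Its construction script creates a dynamic instance of the shared alphabet material on the static mesh's first slot.
; It assigns the alphabet base color, mask and normal textures, then applies the actor's AlphaNumeric metalness, roughness and color variables.
; The event graph holds no active logic.
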(event `self.ReceiveBeginPlay`)

(event `self.ReceiveActorBeginOverlap`
  (params (OtherActor :type "Actor Object Reference")))

(event `self.ReceiveTick`
  (params (DeltaSeconds :type "Float (single-precision)")))

(fn `UserConstructionScript`
  (bind _returnvalue (`PrimitiveComponent.CreateDynamicMaterialInstance` (`self.StaticMesh`) 0 "/Game/ArchVisPolishPack02/Materials/M_AVP2_Alphabet.M_AVP2_Alphabet"))
  (`MaterialInstanceDynamic.SetTextureParameterValue` _returnvalue "Base Color Texture" "/Game/ArchVisPolishPack02/Textures/T_AVP2_Alphabet_D.T_AVP2_Alphabet_D")
  (`MaterialInstanceDynamic.SetTextureParameterValue` _returnvalue "Mask Texture" "/Game/ArchVisPolishPack02/Textures/T_AVP2_Alphabet_M.T_AVP2_Alphabet_M")
  (`MaterialInstanceDynamic.SetTextureParameterValue` _returnvalue "Normal Texture" "/Game/ArchVisPolishPack02/Textures/T_AVP2_Alphabet_N.T_AVP2_Alphabet_N")
  (`MaterialInstanceDynamic.SetScalarParameterValue` _returnvalue "AlphaNumeric.Metalness" (`self.AlphaNumeric.Metalness`))
  (`MaterialInstanceDynamic.SetScalarParameterValue` _returnvalue "AlphaNumeric.Roughness" (`self.AlphaNumeric.Roughness`))
  (`MaterialInstanceDynamic.SetVectorParameterValue` _returnvalue "AlphaNumeric.Color" (`self.AlphaNumeric.Color`)))