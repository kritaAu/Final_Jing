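; Horror enemy AI that chases the player and triggers a jumpscare on contact.
; Pawn sensing sets a never-cleared seen flag, plays a one-time heartbeat and calls FollowPlayer, which moves to the player and plays an attack montage on arrival.
; Sphere overlap with the first-person character fires once, playing a scream and showing the Jump2 widget, then opens MapLevel3 after a short delay.
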(event `self.PawnSensing.OnSeePawn`
  (params (Pawn :type "Pawn Object Reference"))
  (set `self.isSeeingPlayer` true)
  (`self.FollowPlayer`)
  (`/Engine/EditorBlueprintResources/StandardMacros.DoOnce` false
    (:`Completed`
      (`GameplayStatics.PlaySound2D` "/Game/Music/heart-beat-6797.heart-beat-6797" 1.0 1.0 0.0 null null))))

(event `FollowPlayer`
  (set `self.canAttack?` true)
  (if (`self.isSeeingPlayer`)
    (`|AIMoveTo` self (0.0 0.0 0.0) (`GameplayStatics.GetPlayerCharacter` 0) 70.0
      (:`OnSuccess`
        (if (`self.canAttack?`)
          (set `self.canAttack?` false)
          (bind _returnvalue (`self.PlayAnimMontage` "/Game/FirstPersonArms/Animations/FP_Rifle_Shoot_Montage.FP_Rifle_Shoot_Montage"))
          (`KismetSystemLibrary.Delay` _returnvalue)
          (set `self.canAttack?` true))))))

(event `self.Sphere.OnComponentBeginOverlap`
  (params (OverlappedComponent :type "PrimitiveComponent Object Reference") (OtherActor :type "Actor Object Reference") (OtherComp :type "PrimitiveComponent Object Reference") (OtherBodyIndex :type Integer) (bFromSweep :type Boolean) (SweepResult :type "HitResult Structure (by ref)"))
  (cast `/Game/FirstPerson/Blueprints/BP_FirstPersonCharacter` OtherActor)
  (`/Engine/EditorBlueprintResources/StandardMacros.DoOnce` false
    (:`Completed`
      (`GameplayStatics.PlaySoundAtLocation` "/Game/Music/ahhhhhhhh.ahhhhhhhh" (0.0 0.0 0.0) (struct) 1.0 1.0 0.0 null null null null)
      (bind _returnvalue (`|CreateWidget` "/Game/OBJ/jump/jump2.jump2_C"))
      (`UserWidget.AddToViewport` _returnvalue 0)
      (`KismetSystemLibrary.Delay` 0.7)
      (`GameplayStatics.OpenLevel` "MapLevel3"))))

(fn `UserConstructionScript`)